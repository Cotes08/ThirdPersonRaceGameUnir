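; BP_AIPath is a spline path actor that gives AI a target point to follow along a road or track.
; GetClosestLocationToAIPath projects the AI's location onto the spline and advances it by a look-ahead distance.
; The distance wraps past the spline's end so the AI does not brake abruptly on completing a lap.
; The point is then offset along the spline's right vector to the chosen side of the road.
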(event EventBeginPlay)

(event Collision|EventActorBeginOverlap
  (params (OtherActor :type Actor%20Object%20Reference)))

(event EventTick
  (params (DeltaSeconds :type Float%20%28single-precision%29)))

(fn ConstructionScript)

(fn GetClosestLocationtoAIPath
  (params (AILocation :type Vector :default "0, 0, 0") (AdditionalDistance :type Float%20%28double-precision%29) (SideOfRoad :type Integer))
  (bind _spline (Variables|Default|GetSpline))
  (bind _spline_2 (Variables|Default|GetSpline))
  (bind _returnvalue (Class|SplineComponent|GetDistanceAlongSplineatLocation _spline AILocation "World"))
  (bind _returnvalue_2 (Spline|GetSplineLength _spline_2))
  (bind _returnvalue_3 (+ _returnvalue AdditionalDistance))
  (bind _returnvalue_4 (> _returnvalue_3 _returnvalue_2))
  (bind _returnvalue_5 (- _returnvalue_3 _returnvalue_2))
  (bind _returnvalue_6 (Math|Float|SelectFloat _returnvalue_5 _returnvalue_3 _returnvalue_4))
  (return (+ (Spline|GetLocationatDistanceAlongSpline (Variables|Default|GetSpline) _returnvalue_6 "World") (* (Class|SplineComponent|GetRightVectoratDistanceAlongSpline (Variables|Default|GetSpline) _returnvalue_6 "World") (Math|Float|SelectFloat 4.5e+02 -4.5e+02 (Math|Conversions|ToBoolean(Integer) SideOfRoad))))))