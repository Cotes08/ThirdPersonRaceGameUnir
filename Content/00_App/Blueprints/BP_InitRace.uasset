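; BP_InitRace is a trigger box that starts the race for cars and later counts their laps.
; On overlap, input-capable vehicle pawns are started and registered with BP_RacingGameStateBase, which then checks their positions.
; Once the game state's started-car count reaches its car total, further overlaps by input-capable actors update their lap instead.
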(event OnComponentBeginOverlap(Box)
  (params (OverlappedComponent :type Primitive%20Component%20Object%20Reference) (OtherActor :type Actor%20Object%20Reference) (OtherComp :type Primitive%20Component%20Object%20Reference) (OtherBodyIndex :type Integer) (bFromSweep :type Boolean) (SweepResult :type Hit%20Result%20Structure%20%28by%20ref%29))
  (bind _returnvalue (Utilities|DoesObjectImplementInterface OtherActor "/Game/00_App/AI/I_CanReciveInput.I_CanReciveInput_C"))
  (bind _gamestate (Variables|Default|GetGameState))
  (bind _gamestate_2 (Variables|Default|GetGameState))
  ;[1 1 1] Al comenzar vemos que el coche es uno de los que buscamos, en el caso de que si lo guardamos, le seteamos la variable de control de race start y lo registramos en el game state
  (if (> (Variables|/Game/00_App/Blueprints/BP_RacingGameStateBase.BP_RacingGameStateBase_C|GetNumberOfCars _gamestate_2) (Variables|/Game/00_App/Blueprints/BP_RacingGameStateBase.BP_RacingGameStateBase_C|GetCarsStarted _gamestate_2))
    (if _returnvalue
      (bind _asvehicle_adv_pawn (Utilities|Casting|CastToVehicleAdvPawn OtherActor))
      (Utilities|IsValid _asvehicle_adv_pawn
        (:Is%20Valid
          (Default|StartProgress _asvehicle_adv_pawn)
          (Default|RegisterCar _gamestate _asvehicle_adv_pawn)
          (Default|CheckPositions _gamestate _asvehicle_adv_pawn))))
    (elif _returnvalue
      (Default|UpdateLap (Variables|Default|GetGameState) OtherActor))))

(event EventBeginPlay
  (bind _asbp_racing_game_state_base (Utilities|Casting|CastToBP_RacingGameStateBase (Game|GetGameState)))
  (Variables|Default|SetGameState _asbp_racing_game_state_base))

(fn ConstructionScript)